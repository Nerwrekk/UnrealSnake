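; BP_SnakeHead is the snake head actor of a Snake game, with keyboard shortcuts for level and growth control.
; R resets the level through the game mode, G calls GrowSnake, and S casts to SnakeGameModeBase to save, then prints a confirmation.
; The construction script is empty; its disconnected logic for building spline mesh segments between spline points never runs.
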(event `Key|R`
  (params (Key :type "Key Structure"))
  (:`Pressed`
    (`GameModeBase.ResetLevel` (`GameplayStatics.GetGameMode`))))

(event `Key|G`
  (params (Key :type "Key Structure"))
  (:`Pressed`
    (`self.GrowSnake`)))

(event `Key|S`
  (params (Key :type "Key Structure"))
  (:`Pressed`
    (bind _assnake_game_mode_base (cast `SnakeGameModeBase` (`GameplayStatics.GetGameMode`)))
    (`SnakeGameModeBase.SaveGame` _assnake_game_mode_base)
    (`KismetSystemLibrary.PrintString` "Saved Game")))

(fn `UserConstructionScript`)