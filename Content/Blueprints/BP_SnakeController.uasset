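; Controller for the Snake game that puts the score HUD on screen and refreshes it.
; On BeginPlay, it confirms the player pawn is a SnakeHead, then creates WBP_UserInterface and adds it to the viewport.
; It writes Score and HighScore into the widget's labeled text fields, and the UpdateScore event re-runs that same text update on the existing widget.
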(event `self.ReceiveBeginPlay`
  (cast `SnakeHead` (`GameplayStatics.GetPlayerPawn` 0))
  (bind _returnvalue (`|CreateWidget` "/Game/Blueprints/Widgets/WBP_UserInterface.WBP_UserInterface_C"))
  (`UserWidget.AddToViewport` _returnvalue 0)
  (`TextBlock.SetText` (`/Game/Blueprints/Widgets/WBP_UserInterface.Score` _returnvalue) (`KismetTextLibrary.Conv_StringToText` (`KismetStringLibrary.Concat_StrStr` "Score: " (`KismetTextLibrary.Conv_TextToString` (`KismetTextLibrary.Conv_IntToText` (`self.Score`))))) :!label _label)
  (`TextBlock.SetText` (`/Game/Blueprints/Widgets/WBP_UserInterface.HighScore` _returnvalue) (`KismetTextLibrary.Conv_StringToText` (`KismetStringLibrary.Concat_StrStr` "HighScore: " (`KismetTextLibrary.Conv_TextToString` (`KismetTextLibrary.Conv_IntToText` (`self.HighScore`)))))))

(event `self.UpdateScore`
  (goto _label))

(fn `UserConstructionScript`)