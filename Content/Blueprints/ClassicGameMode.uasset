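; ClassicGameMode is the game mode for a snake game's classic mode, handling the start menu and game-over score entry.
; On BeginPlay it shows the start menu widget and enables the mouse cursor for the first player controller.
; Its GameOver event casts the given controller to SnakeController, then opens a score entry widget owned by that controller, passing in and displaying its score.
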(event `self.ReceiveBeginPlay`
  (bind _returnvalue (`|CreateWidget` "/Game/Blueprints/Widgets/WBP_StartMenu.WBP_StartMenu_C"))
  (`UserWidget.AddToViewport` _returnvalue 0)
  (set `PlayerController.bShowMouseCursor` true (`GameplayStatics.GetPlayerController` 0)))

(event `self.GameOver`
  (params (Controller :type "Controller Object Reference"))
  (bind _assnake_controller (cast `SnakeController` Controller))
  (bind _returnvalue (`|CreateWidget` "/Game/Blueprints/Widgets/WBP_EnterScore.WBP_EnterScore_C" _assnake_controller))
  (bind _score (`SnakeController.Score` _assnake_controller))
  (set `/Game/Blueprints/Widgets/WBP_EnterScore.Score` _score _returnvalue)
  (`UserWidget.AddToViewport` _returnvalue 0)
  (`TextBlock.SetText` (`/Game/Blueprints/Widgets/WBP_EnterScore.ScoreText` _returnvalue) (`KismetTextLibrary.Conv_StringToText` (`KismetStringLibrary.Concat_StrStr` "Your score: " (`KismetTextLibrary.Conv_TextToString` (`KismetTextLibrary.Conv_IntToText` _score))))))

(fn `UserConstructionScript`)